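; BP_Rifle is a hitscan rifle actor fired through its PullTrigger event.
; PullTrigger attaches a Niagara muzzle flash to the mesh's Muzzle socket, then traces from the owning pawn's controller view point out to MaxRange.
; On a hit, it spawns an impact effect and binds an empty DamageEvent to the hit actor's OnTakeAnyDamage, without applying any damage.
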(event `self.PullTrigger`
  (`NiagaraFunctionLibrary.SpawnSystemAttached` "/Game/MuzzleFlash/NS_MuzzleFlash_Rifle.NS_MuzzleFlash_Rifle" (`self.Mesh`) "Muzzle" (0.0 0.0 0.0) (struct :`Yaw` -90.0) "KeepRelativeOffset" true)
  (bind _aspawn (cast `Pawn` (`self.GetOwner`)))
  (bind (_location _rotation) (`Controller.GetPlayerViewPoint` (`Pawn.GetController` _aspawn)))
  (bind (_outhit _returnvalue) (`KismetSystemLibrary.LineTraceSingle` _location (+ (* (`self.MaxRange`) (`KismetMathLibrary.Conv_RotatorToVector` _rotation)) _location) "TraceTypeQuery3"))
  (if _returnvalue
    (`NiagaraFunctionLibrary.SpawnSystemAtLocation` "/Game/MuzzleFlash/NS_Muzzle_Flash_Impact.NS_Muzzle_Flash_Impact" (`.Location` (`GameplayStatics.BreakHitResult` _outhit)) (`KismetMathLibrary.ComposeRotators` _rotation (struct :`Yaw` 90.0)))
    (add `self.OnTakeAnyDamage` (`.HitActor` (`GameplayStatics.BreakHitResult` _outhit)) (delegate `DamageEvent`))))

(event `DamageEvent` :!signature `self.OnTakeAnyDamage`
  (params (DamagedActor :type "Actor Object Reference") (Damage :type "Float (single-precision)") (DamageType :type "DamageType Object Reference") (InstigatedBy :type "Controller Object Reference") (DamageCauser :type "Actor Object Reference")))

(fn `UserConstructionScript`)